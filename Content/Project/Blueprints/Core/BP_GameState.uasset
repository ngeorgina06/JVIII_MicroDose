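; Game state Blueprint that runs a three-minute countdown and decides when the match ends for two characters.
; Tick derives elapsed and remaining time from the start timestamp, ending the match when time runs out.
; Each character's finish records its time once; the match also ends when both have finished.
; Either ending flags the game over and shows the WBP_MenuFin end menu once for player 0.
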(event EventBeginPlay
  ;[0.15 0.15 0.15 0.5] Activer chrono
  (Variables|Default|SetTempsInitial 1.8e+02)
  (Variables|Default|SetTempsRestant 1.8e+02)
  (Variables|Default|SetTempsEcoule 0.0)
  (Variables|Default|SetChronoActif true)
  (Variables|Default|SetTempsDebut (Utilities|Time|GetGameTimeinSeconds)))

(event EventTick
  (params (DeltaSeconds :type Float%20%28single-precision%29))
  ;[0.15 0.15 0.15 0.5] Chronometre system
  (if (Variables|Default|GetChronoActif)
    (Variables|Default|SetTempsEcoule (- (Utilities|Time|GetGameTimeinSeconds) (Variables|Default|GetTempsDebut)))
    (Variables|Default|SetTempsRestant (Math|Float|Max(Float) (- (Variables|Default|GetTempsInitial) (Variables|Default|GetTempsEcoule)) 0.0))
    (if (<= (Variables|Default|GetTempsRestant) 0.0)
      (Variables|Default|SetChronoActif false)
      (Variables|Default|SetTempsRestant 0.0)
      (CallFunction|TerminerPartieTempsEcoule))))

(fn ConstructionScript)

(fn TerminerPersonnage1
  (if (not (Variables|Default|GetPersonnage1Termine))
    (Variables|Default|SetTempsPersonnage1 (Variables|Default|GetTempsEcoule))
    (Variables|Default|SetPersonnage1Termine true)
    (CallFunction|VerifierFinPartie)))

(fn TerminerPersonnage2
  (if (not (Variables|Default|GetPersonnage2Termine))
    (Variables|Default|SetTempsPersonnage2 (Variables|Default|GetTempsEcoule))
    (Variables|Default|SetPersonnage2Termine true)
    (CallFunction|VerifierFinPartie)))

(fn VerifierFinPartie
  (if (and (Variables|Default|GetPersonnage1Termine) (Variables|Default|GetPersonnage2Termine))
    (Variables|Default|SetPartieTerminee true)
    (CallFunction|AfficherFinPartie)))

(fn TerminerPartieTempsEcoule
  (Variables|Default|SetChronoActif false)
  (Variables|Default|SetTempsRestant 0.0)
  (Variables|Default|SetPartieTerminee true)
  (CallFunction|AfficherFinPartie))

(fn AfficherFinPartie
  (if (not (Variables|Default|GetWidgetFinPartieAffiche))
    (bind _returnvalue (UserInterface|CreateWidget "/Game/Project/UI/Blueprints/WBP_MenuFin.WBP_MenuFin_C" (Game|GetPlayerController 0)))
    (UserInterface|Viewport|AddtoViewport _returnvalue 0)
    (Variables|Default|SetWidgetFinPartieAffiche true)))