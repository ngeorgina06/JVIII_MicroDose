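; Player component for BP_FirstPersonCharacter that provides camera-based traces for interaction and bullet impacts.
; It caches the owning character on BeginPlay and traces forward from its camera on the Visibility channel.
; LineTrace returns the hit actor only if it implements BPI_Interactible, and leaves debug drawing on.
; FireTrace spawns a random, randomly sized, short-lived impact decal without checking for a hit, and applies no damage.
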(event EventBeginPlay
  (bind _asbp_first_person_character (Utilities|Casting|CastToBP_FirstPersonCharacter (Components|GetOwner)))
  (Variables|Default|SetPlayerRef _asbp_first_person_character))

(fn LineTrace
  (params (Length :type Float%20%28double-precision%29))
  (bind _playerref (Variables|Default|GetPlayerRef))
  (bind _firstpersoncamera (Variables|/Game/Project/Blueprints/Characters/Player/BP_FirstPersonCharacter.BP_FirstPersonCharacter_C|GetFirstPersonCamera _playerref))
  (bind _returnvalue (Transformation|GetWorldLocation _firstpersoncamera))
  (bind _outhit (Collision|LineTraceByChannel _returnvalue (+ _returnvalue (* (Math|Vector|GetForwardVector _firstpersoncamera) Length)) "TraceTypeQuery1" false 0 "ForDuration" true "(R=1.000000,G=0.017220,B=0.362525,A=1.000000)" "(R=1.000000,G=0.000000,B=0.019773,A=1.000000)"))
  (if (and (Utilities|IsValid (.HitActor (Collision|BreakHitResult _outhit))) (Utilities|DoesObjectImplementInterface (.HitActor (Collision|BreakHitResult _outhit)) "/Game/Project/Blueprints/Interfaces/BPI_Interactible.BPI_Interactible_C"))
    (return (.HitActor (Collision|BreakHitResult _outhit)))
    (else
      (return 0))))

(fn FireTrace
  (params (Length :type Float%20%28double-precision%29))
  (bind _playerref (Variables|Default|GetPlayerRef))
  (bind _firstpersoncamera (Variables|/Game/Project/Blueprints/Characters/Player/BP_FirstPersonCharacter.BP_FirstPersonCharacter_C|GetFirstPersonCamera _playerref))
  (bind _returnvalue (Transformation|GetWorldLocation _firstpersoncamera))
  (bind _outhit (Collision|LineTraceByChannel _returnvalue (+ _returnvalue (* (Math|Vector|GetForwardVector _firstpersoncamera) Length)) "TraceTypeQuery1" false 0 "None" true "(R=1.000000,G=0.017220,B=0.362525,A=1.000000)" "(R=1.000000,G=0.000000,B=0.019773,A=1.000000)"))
  (Rendering|Decal|SpawnDecalatLocation (.OutItem (Utilities|Array|Random (Variables|Default|GetBulletImpactMat))) (Math|Conversions|ToVector(Float) (Math|Random|RandomFloatinRange 5.0 1e+01)) (.ImpactPoint (Collision|BreakHitResult _outhit)) (Math|Rotator|FindLookatRotation (.TraceStart (Collision|BreakHitResult _outhit)) (.TraceEnd (Collision|BreakHitResult _outhit))) 8.0))