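; Enemy NPC character that patrols and reacts to what its AI Perception senses.
; Patrol loops AIMoveTo and a wait, picking either random reachable points around the start location or tagged path actors, in order or at random.
; A "MakingNoise" stimulus sends it to that location; other stimuli make it chase the first-person player at speed 500.
; Forgetting the target resumes patrol at that same speed; the construction script previews the radius.
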(event OnTargetPerceptionUpdated(AIPerception)
  (params (Actor :type Actor%20Object%20Reference) (Stimulus :type AI%20Stimulus%20Structure))
  (bind (_age _expirationage _strength _stimuluslocation _receiverlocation _tag _bsuccessfullysensed) (Utilities|Struct|BreakAIStimulus Stimulus))
  ;[0.8152 0 1 0.5] Lordque le personnage ennemi me voit
  (if _bsuccessfullysensed
    (if (not (== _tag "MakingNoise"))
      ;;[1 0.546 0.2068 0.5] Le NPC court vers le joueur
      ;;;[0.15 0.15 0.15 0.5] Tag recherche prend du temps et == au personnage aussi. Utiliser cela
      (bind _asbp_first_person_character (Utilities|Casting|CastToBP_FirstPersonCharacter Actor))
      ;;;[0.15 0.15 0.15 0.5] Changer une variable (drag-drop thing + set)
      (Variables|/Script/Engine.CharacterMovementComponent|SetMaxWalkSpeed (Variables|Character|GetCharacterMovement) 5e+02)
      (AI|AIMoveTo self "0, 0, 0" _asbp_first_person_character 5.0 false)
      (else
        (AI|AIMoveTo self _stimuluslocation 0 5.0 false)))))

(event OnTargetPerceptionForgotten(AIPerception)
  (params (Actor :type Actor%20Object%20Reference))
  ;[0 0.7603 1 0.5] Lorsque le personnage me perd
  (Variables|/Script/Engine.CharacterMovementComponent|SetMaxWalkSpeed (Variables|Character|GetCharacterMovement) 5e+02)
  (CallFunction|Patrol))

(event Custom|Patrol
  ;[0.3415 1 0 0.5] Faire bouger le personnage
  (bind _destination (CallFunction|CalculateDestination))
  ;;[0.15 0.15 0.15 0.5] Fonction prend du temps
  (AI|AIMoveTo self _destination 0 5.0 false
    (:OnSuccess
      (Utilities|FlowControl|Delay (Variables|Default|GetPatrolWaitTime))
      (CallFunction|Patrol))))

(event EventBeginPlay
  ;[1 0.05761 0 0.5] Permet au personnage Enemy de récupérer les points qu'ils peut
  ; patrouiller selon un tag spécifique (ici Path01) et ensuite, lance la boucle qui permet au personnage de se déplacer
  (Variables|Default|SetStartLocation (Transformation|GetActorLocation))
  (bind _outactors (Actor|GetAllActorswithTag (Variables|Default|GetPathTag)))
  (Variables|Default|SetPatrolPaths _outactors)
  (CallFunction|Patrol))

(fn ConstructionScript
  (if (Variables|Default|GetShowPatrolRadius)
    (Rendering|SetVisibility (Variables|Default|GetDrawPatrolRadius) true false)
    (Components|Sphere|SetSphereRadius (Variables|Default|GetDrawPatrolRadius) (Variables|Default|GetPatrolRadius) true)
    (else
      (Rendering|SetVisibility (Variables|Default|GetDrawPatrolRadius) false false))))

(fn CalculateDestination
  (if (Variables|Default|GetPatrolByRadius)
    (LocalVariables|SetLocalDestination (.RandomLocation (AI|Navigation|GetRandomReachablePointinRadius (Variables|Default|GetStartLocation) (Variables|Default|GetPatrolRadius) 0 0)))
    (return (LocalVariables|GetLocalDestination))
    (elif (> (Utilities|Array|Length (Variables|Default|GetPatrolPaths)) 0)
      (if (Variables|Default|GetIsRandomPath)
        (LocalVariables|SetLocalDestination (Transformation|GetActorLocation (.OutItem (Utilities|Array|Random (Variables|Default|GetPatrolPaths)))))
        (else
          (LocalVariables|SetLocalDestination (Transformation|GetActorLocation (Utilities|Array|Get(acopy) (Variables|Default|GetPatrolPaths) (Variables|Default|GetCurrentPathIndex))))
          (Variables|Default|SetCurrentPathIndex (Math|Integer|%(Integer) (+ (Variables|Default|GetCurrentPathIndex) 1) (Utilities|Array|Length (Variables|Default|GetPatrolPaths))))))
      (return (LocalVariables|GetLocalDestination)))))